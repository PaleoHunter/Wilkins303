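; BP_Turret is an enemy turret that tracks and shoots at the player while they are inside its detection Box.
; Overlap of a BP_PlayerChar starts two looping timers by function name, and leaving the box clears both.
; One timer rapidly snaps the Pivot to look at player 0 from the actor's location.
; The other periodically spawns a BP_Turretprojectile at the ProjectileSpawn transform.
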(event `FallowsPlayer`
  (`SceneComponent.K2_SetWorldRotation` (`self.Pivot`) (`KismetMathLibrary.FindLookAtRotation` (`self.K2_GetActorLocation`) (`self.K2_GetActorLocation` (`GameplayStatics.GetPlayerCharacter` 0))) false false))

(event `FireAtPlayer`
  (`|SpawnActorFromClass` "/Game/Enemy/Turret/BP_Turretprojectile.BP_Turretprojectile_C" (`SceneComponent.K2_GetComponentToWorld` (`self.ProjectileSpawn`)) "Undefined" "MultiplyWithRoot" null null))

(event `self.Box.OnComponentBeginOverlap`
  (params (OverlappedComponent :type "PrimitiveComponent Object Reference") (OtherActor :type "Actor Object Reference") (OtherComp :type "PrimitiveComponent Object Reference") (OtherBodyIndex :type Integer) (bFromSweep :type Boolean) (SweepResult :type "HitResult Structure (by ref)"))
  (cast `/Game/Player/BP_PlayerChar` OtherActor)
  (`KismetSystemLibrary.K2_SetTimer` null "FallowsPlayer" 0.05 true)
  (`KismetSystemLibrary.K2_SetTimer` null "FireAtPlayer" 0.5 true))

(event `self.Box.OnComponentEndOverlap`
  (params (OverlappedComponent :type "PrimitiveComponent Object Reference") (OtherActor :type "Actor Object Reference") (OtherComp :type "PrimitiveComponent Object Reference") (OtherBodyIndex :type Integer))
  (cast `/Game/Player/BP_PlayerChar` OtherActor)
  (`KismetSystemLibrary.K2_ClearTimer` null "FallowsPlayer")
  (`KismetSystemLibrary.K2_ClearTimer` null "FireAtPlayer"))

(fn `UserConstructionScript`)